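; BP_Gun is a gun pickup that registers itself with the first-person player who touches it.
; Its Sphere overlap checks for the Player tag, casts to BP_FirstPersonCharacter and fetches that character's AC_WeaponThrowables component.
; It sets itself as that component's GunItem and CurrentItem, then hides in game rather than being destroyed, so the stored references stay valid.
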(event OnComponentBeginOverlap(Sphere)
  (params (OverlappedComponent :type Primitive%20Component%20Object%20Reference) (OtherActor :type Actor%20Object%20Reference) (OtherComp :type Primitive%20Component%20Object%20Reference) (OtherBodyIndex :type Integer) (bFromSweep :type Boolean) (SweepResult :type Hit%20Result%20Structure%20%28by%20ref%29))
  (bind _self self)
  (if (Actor|ActorHasTag OtherActor "Player")
    (bind _asbp_first_person_character (Utilities|Casting|CastToBP_FirstPersonCharacter OtherActor))
    (bind _output_get (Variables|Default|SetAs%20AC%20Weapon%20Throwables (Actor|GetComponentbyClass _asbp_first_person_character "/Game/Weapon_Throwables/AC_WeaponThrowables.AC_WeaponThrowables_C")))
    (Variables|/Game/Weapon_Throwables/AC_WeaponThrowables.AC_WeaponThrowables_C|SetGunItem _output_get _self)
    (Variables|/Game/Weapon_Throwables/AC_WeaponThrowables.AC_WeaponThrowables_C|SetCurrentItem _output_get _self)
    (Rendering|SetActorHiddenInGame true)))

(fn ConstructionScript
  (|CallParentFunction))