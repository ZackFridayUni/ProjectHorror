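; BP_GunItem is a gun pickup that equips itself to the first-person character who walks into it.
; On overlap it zeroes its sphere trigger, registers itself as the character's GunItem and CurrentItem, and snaps onto the GripPoint socket of the first-person mesh.
; It then adds the IMC_Weapons Enhanced Input mapping context to that player's local subsystem.
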(event OnComponentBeginOverlap(Sphere)
  (params (OverlappedComponent :type Primitive%20Component%20Object%20Reference) (OtherActor :type Actor%20Object%20Reference) (OtherComp :type Primitive%20Component%20Object%20Reference) (OtherBodyIndex :type Integer) (bFromSweep :type Boolean) (SweepResult :type Hit%20Result%20Structure%20%28by%20ref%29))
  (bind _self self)
  (Components|Sphere|SetSphereRadius (Variables|Default|GetSphere) 0.0 true)
  (bind _asbp_first_person_character (Utilities|Casting|CastToBP_FirstPersonCharacter OtherActor))
  (bind _output_get (Variables|Default|SetFirstPersonCharacterRef _asbp_first_person_character))
  (Variables|/Game/FirstPerson/Blueprints/BP_FirstPersonCharacter.BP_FirstPersonCharacter_C|SetGunItem _output_get _self)
  (Variables|/Game/FirstPerson/Blueprints/BP_FirstPersonCharacter.BP_FirstPersonCharacter_C|SetCurrentItem _output_get _self)
  (Transformation|AttachComponentToComponent (Variables|/Game/FirstPerson/Blueprints/BP_FirstPersonCharacter.BP_FirstPersonCharacter_C|GetFirstPersonMesh _output_get) "GripPoint" "SnapToTarget" "SnapToTarget" "KeepWorld" true)
  (bind _asplayer_controller (Utilities|Casting|CastToPlayerController (Pawn|GetController _output_get)))
  (Utilities|IsValid (PlayerController|LocalPlayerSubsystems|GetEnhancedInputLocalPlayerSubsystem _asplayer_controller)
    (:Is%20Valid
      (Input|AddMappingContext (PlayerController|LocalPlayerSubsystems|GetEnhancedInputLocalPlayerSubsystem _asplayer_controller) "/Game/FirstPerson/Input/IMC_Weapons.IMC_Weapons" 1 "(bIgnoreAllPressedKeysUntilRelease=True,bForceImmediately=False,bNotifyUserSettings=False)"))))

(fn ConstructionScript
  (|CallParentFunction))