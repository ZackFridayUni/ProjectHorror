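; Weapon component for the first-person player that switches between a gun and a throwable item, with a predicted throw arc.
; A looping timer predicts the projectile path from the camera, feeds it into the character's spline and calls for spline meshes.
; The throw (impulse-launched spawn), hitscan shot with damage and shake, arc trigger and mesh placement are all unwired, so only item selection responds to input.
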(event Custom|Draw%20Projectile%20Curve
  (bind _returnvalue (Utilities|Time|SetTimerbyEvent (delegate Custom|Update%20Projectile%20Curve) 0.01 true))
  (Variables|Default|SetProjectileCurveTimer _returnvalue))

(event Custom|Update%20Projectile%20Curve
  (bind _returnvalue (Game|GetPlayerCameraManager 0))
  (bind _returnvalue_2 (Camera|GetCameraRotation _returnvalue))
  (bind _returnvalue_3 (Math|Vector|GetForwardVector _returnvalue_2))
  (bind _returnvalue_4 (* _returnvalue_3 1e+03))
  (bind (_x _y) (Math|Vector|BreakVector _returnvalue_4))
  (CallFunction|ClearSplinePoint)
  (bind _asbp_first_person_character (Utilities|Casting|CastToBP_FirstPersonCharacter (Game|Player|GetPlayerPawn 0)))
  (bind _predictresult (Class|GameplayStatics|BlueprintPredictProjectilePathAdvanced (Utilities|Struct|MakePredictProjectilePathParams (Transformation|GetWorldLocation (Variables|/Game/StudentWork/Blueprints/Player/BP_FirstPersonCharacter.BP_FirstPersonCharacter_C|GetFirstPersonCamera _asbp_first_person_character)) (Math|Vector|MakeVector _x _y (* (Math|Float|MapRangeUnclamped (.Z (Math|Vector|BreakVector _returnvalue_3)) 0.0 1.0 3.0 1e+01) 5e+01)) true 0.0 1.0 true "ECC_WorldStatic" "ObjectTypeQuery1" (Utilities|Array|MakeArray _asbp_first_person_character) 13.0 0.0 "ForDuration" 5.0 false)))
  (for _array_element (.PathData (Utilities|Struct|BreakPredictProjectilePathResult _predictresult))
    (Spline|AddSplinePoint (Variables|/Game/StudentWork/Blueprints/Player/BP_FirstPersonCharacter.BP_FirstPersonCharacter_C|GetProjectile%20Spline _asbp_first_person_character) (.Location (Utilities|Struct|BreakPredictProjectilePathPointData _array_element)) "World" true))
  (for _index (range 1 (Spline|GetNumberOfSplinePoints (Variables|/Game/StudentWork/Blueprints/Player/BP_FirstPersonCharacter.BP_FirstPersonCharacter_C|GetProjectile%20Spline _asbp_first_person_character)))
    (Default|CallAddSplineMesh)))

(event Custom|Clear%20Spline%20Point
  (Components|DestroyComponent)
  (Utilities|Array|Clear (Variables|Default|GetSpline%20Mesh)))

(event Input|ActionEvents|InputActionGunSelect
  (params (Key :type Key%20Structure))
  (:Pressed
    (Variables|Default|SetCurrentItem (Variables|Default|GetGunItem))))

(event Input|ActionEvents|InputActionThrowableSelect
  (params (Key :type Key%20Structure))
  (:Pressed
    (Variables|Default|SetCurrentItem (Variables|Default|GetThrowableItem))))

(event Input|ActionEvents|InputActionShootThrow
  (params (Key :type Key%20Structure)))

(event Input|ActionEvents|InputActionShootThrow
  (params (Key :type Key%20Structure)))