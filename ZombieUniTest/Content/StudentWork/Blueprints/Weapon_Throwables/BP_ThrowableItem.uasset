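; BP_ThrowableItem is a physics-simulated world item that registers itself as the player's throwable on contact.
; Its static mesh starts simulating physics on BeginPlay.
; When BP_FirstPersonCharacter begins overlapping its sphere, it writes its own class into the character's ThrowableItem and itself into CurrentItem.
; It contains no throw or end-overlap logic.
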(event OnComponentBeginOverlap(Sphere)
  (params (OverlappedComponent :type Primitive%20Component%20Object%20Reference) (OtherActor :type Actor%20Object%20Reference) (OtherComp :type Primitive%20Component%20Object%20Reference) (OtherBodyIndex :type Integer) (bFromSweep :type Boolean) (SweepResult :type Hit%20Result%20Structure%20%28by%20ref%29))
  (bind _self self)
  (bind _asbp_first_person_character (Utilities|Casting|CastToBP_FirstPersonCharacter OtherActor))
  (bind _output_get (Variables|Default|SetAs%20BP%20First%20Person%20Character _asbp_first_person_character))
  (Variables|/Game/StudentWork/Blueprints/Player/BP_FirstPersonCharacter.BP_FirstPersonCharacter_C|SetThrowableItem _output_get (Utilities|GetClass _self))
  (Variables|/Game/StudentWork/Blueprints/Player/BP_FirstPersonCharacter.BP_FirstPersonCharacter_C|SetCurrentItem _output_get _self))

(event EventBeginPlay
  (Physics|SetSimulatePhysics (Variables|Default|GetStaticMesh) true))

(fn ConstructionScript
  (|CallParentFunction))