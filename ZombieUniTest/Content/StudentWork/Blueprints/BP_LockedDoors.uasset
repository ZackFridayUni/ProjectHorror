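; BP_LockedDoors is a door actor that opens for a player carrying a keycard by destroying itself.
; When the first-person character begins overlapping it, its IsKeycardObtained flag decides between destroying the door and showing a WB_LockedDoors widget on screen.
; When a character without the keycard stops overlapping, that stored widget is removed from the viewport.
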(event EventBeginPlay)

(event Collision|EventActorBeginOverlap
  (params (OtherActor :type Actor%20Object%20Reference))
  (bind _asbp_first_person_character (Utilities|Casting|CastToBP_FirstPersonCharacter OtherActor))
  (if (Variables|/Game/StudentWork/Blueprints/Player/BP_FirstPersonCharacter.BP_FirstPersonCharacter_C|GetIsKeycardObtained? _asbp_first_person_character)
    (Actor|DestroyActor)
    (else
      (bind _returnvalue (UserInterface|CreateWidget "/Game/StudentWork/Blueprints/WB_LockedDoors.WB_LockedDoors_C"))
      (bind _output_get (Variables|Default|SetWidget _returnvalue))
      (UserInterface|Viewport|AddtoViewport _output_get 0))))

(event EventTick
  (params (DeltaSeconds :type Float%20%28single-precision%29)))

(event Collision|EventActorEndOverlap
  (params (OtherActor :type Actor%20Object%20Reference))
  (bind _asbp_first_person_character (Utilities|Casting|CastToBP_FirstPersonCharacter OtherActor))
  (if (not (Variables|/Game/StudentWork/Blueprints/Player/BP_FirstPersonCharacter.BP_FirstPersonCharacter_C|GetIsKeycardObtained? _asbp_first_person_character))
    (Widget|RemovefromParent (Variables|Default|GetWidget))))

(fn ConstructionScript)