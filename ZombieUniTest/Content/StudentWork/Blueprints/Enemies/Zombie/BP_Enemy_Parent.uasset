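; Parent Blueprint for zombie enemies that handles taking damage and dying.
; AnyDamage subtracts from CurrentHealth and sets IsDead only when health equals exactly zero, with no clamping.
; On death it clears the WalkToLocationTime timer, disables character movement and plays a non-looping death animation on the mesh.
; A getter function returns a reference to the enemy itself.
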(event Game|Damage|EventAnyDamage
  (params (Damage :type Float%20%28single-precision%29) (DamageType :type Damage%20Type%20Object%20Reference) (InstigatedBy :type Controller%20Object%20Reference) (DamageCauser :type Actor%20Object%20Reference))
  ;[1 1 1] Take Damage
  (Variables|Default|SetCurrentHealth (- (Variables|Default|GetCurrentHealth) Damage))
  (bind _output_get (Variables|Default|SetIsDead (== (Variables|Default|GetCurrentHealth) 0.0)))
  (if _output_get
    (Utilities|Time|ClearandInvalidateTimerbyHandle (Variables|Default|GetWalk%20To%20Location%20Time))
    (Pawn|Components|CharacterMovement|DisableMovement (Variables|Character|GetCharacterMovement))
    (Components|Animation|PlayAnimation (Variables|Character|GetMesh) "/Game/StudentWork/Blueprints/Enemies/Zombie/Animation/Death/Zombie_Death.Zombie_Death" false)))

(fn ConstructionScript)

(fn GetEnemyRefrence
  (return self))