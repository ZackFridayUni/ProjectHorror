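; Noise-triggered zombie enemy that starts without patrolling, plays looping breathing audio, and reacts to sounds heard through PawnSensing.
; Each noise attempts a melee montage if the player overlaps AttackRange, with a notify-driven sphere trace applying damage.
; It also starts a repeating timer that reissues AIMoveTo toward the sound.
; After arriving, or failing nearby with the player crouched, it waits, gets bored and roams random reachable points.
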(event OnHearNoise(PawnSensing)
  (params (Instigator :type Pawn%20Object%20Reference) (Location :type Vector%20%28by%20ref%29 :default "0, 0, 0") (Volume :type Float%20%28single-precision%29))
  ;[1 1 1] Main
  (if (not (Variables|Default|GetIsDead))
    (Variables|Default|SetSound%20Location Location)
    (Variables|Default|SetHeard true)
    (Development|PrintString "Heard")
    (CallFunction|Attack)
    (CallFunction|GotoLocationOfSound)))

(event OnComponentBeginOverlap(AttackRange)
  (params (OverlappedComponent :type Primitive%20Component%20Object%20Reference) (OtherActor :type Actor%20Object%20Reference) (OtherComp :type Primitive%20Component%20Object%20Reference) (OtherBodyIndex :type Integer) (bFromSweep :type Boolean) (SweepResult :type Hit%20Result%20Structure%20%28by%20ref%29))
  ;[1 1 1] Check If Player Is Nearby
  (Utilities|Casting|CastToBP_FirstPersonCharacter OtherActor)
  (Variables|Default|SetInRange? true))

(event OnComponentEndOverlap(AttackRange)
  (params (OverlappedComponent :type Primitive%20Component%20Object%20Reference) (OtherActor :type Actor%20Object%20Reference) (OtherComp :type Primitive%20Component%20Object%20Reference) (OtherBodyIndex :type Integer))
  ;[1 1 1] Check If Player Is Nearby
  (Variables|Default|SetInRange? false))

(event Custom|Following
  (bind _acceptance_radius (Variables|Default|GetAcceptance%20Radius))
  ;[1 1 1] Go to Location of Sound
  (AI|AIMoveTo self (Variables|Default|GetSound%20Location) 0 _acceptance_radius false
    (:then
      (Variables|/Script/Engine.CharacterMovementComponent|SetMaxWalkSpeed (Variables|Character|GetCharacterMovement) (Variables|Default|GetSpeed%20to%20reach%20sound%20location)))
    (:OnSuccess
      (Development|PrintString "Here")
      (Utilities|FlowControl|Delay (Variables|Default|GetTime%20Before%20Bored) :!label _label)
      (Development|PrintString "Bored")
      (Variables|Default|SetHeard false)
      (CallFunction|Bored))
    (:OnFail
      (bind _returnvalue (Actor|GetActorOfClass "/Game/StudentWork/Blueprints/Player/BP_FirstPersonCharacter.BP_FirstPersonCharacter_C"))
      (if (< (Math|Vector|Distance(Vector) (Transformation|GetActorLocation) (Variables|Default|GetSound%20Location)) (* _acceptance_radius 2.0))
        (if (not (Variables|/Script/Engine.Character|GetbIsCrouched _returnvalue))
          (Development|PrintString "Still Heard")
          (else
            (Development|PrintString "Failed 2x")
            (goto _label)))))))

(event Custom|Go%20to%20Location%20of%20Sound
  ;[1 1 1] Go to Location of Sound
  (if (not (Variables|Default|GetIsDead))
    (Utilities|Time|ClearandInvalidateTimerbyHandle (Variables|Default|GetTime%20to%20reach%20random%20location))
    (bind _returnvalue (Utilities|Time|SetTimerbyEvent (delegate Custom|Following) 0.1 true))
    (Variables|Default|SetWalk%20To%20Location%20Time _returnvalue)))

(event Custom|Attack
  (bind _returnvalue (Transformation|GetActorLocation))
  (if (not (Variables|Default|GetIsDead))
    (bind _returnvalue_2 (Actor|GetActorOfClass "/Game/StudentWork/Blueprints/Player/BP_FirstPersonCharacter.BP_FirstPersonCharacter_C"))
    ;[1 1 1] Attack
    (if (Math|Boolean|ANDBoolean (Variables|Default|GetCan%20Attack?) (Variables|Default|GetHeard) (Utilities|Array|ContainsItem (Collision|GetOverlappingActors (Variables|Default|GetAttack%20Range) "/Game/StudentWork/Blueprints/Player/BP_FirstPersonCharacter.BP_FirstPersonCharacter_C" :!class /Script/Engine.PrimitiveComponent) _returnvalue_2))
      (Animation|Montage|PlayMontage (Variables|Character|GetMesh) "/Game/StudentWork/Blueprints/Enemies/Zombie/Animation/Bite/Zombie_Attack_Montage.Zombie_Attack_Montage"
        (:then
          (Variables|Default|SetCan%20Attack? false))
        (:OnCompleted
          (Variables|Default|SetCan%20Attack? true :!label _label))
        (:OnInterrupted
          (goto _label))
        (:OnNotifyBegin
          (bind (_outhit _returnvalue_3) (Collision|SphereTraceForObjects _returnvalue (+ _returnvalue (* (Math|Vector|GetForwardVector (Transformation|GetActorRotation)) 2e+02)) 0.0 (Utilities|Array|MakeArray "ObjectTypeQuery3") false 0 "None"))
          (if _returnvalue_3
            (Game|Damage|ApplyDamage (.HitActor (Collision|BreakHitResult _outhit)) 1e+01 0 0)
            (Variables|Default|SetOverlap false)
            (Audio|PlaySoundatLocation "/Game/StudentWork/Assets/SFX/Enemy/Enemy_Hitting_Player_Cue.Enemy_Hitting_Player_Cue" (Transformation|GetActorLocation) "0, 0, 0" 1.0 1.0 0.0 0 0 0 0)))))))

(event Custom|StartBreathing
  (CallFunction|Breathing)
  (Utilities|Time|SetTimerbyEvent (delegate Custom|Breathing) 14.0 true))

(event Custom|Bored
  (Utilities|Time|ClearandInvalidateTimerbyHandle (Variables|Default|GetWalk%20To%20Location%20Time))
  (CallFunction|Patrol))

(event Custom|Breathing
  (Audio|PlaySoundatLocation "/Game/StudentWork/Assets/SFX/Player/EnemyBreathing.EnemyBreathing" (Transformation|GetActorLocation) "0, 0, 0" 0.75 0.5 0.0 0 0 0 0))

(event Custom|Patrol
  ;[1 1 1] Roam Movement
  (if (not (Variables|Default|GetIsDead))
    (AI|AIMoveTo self (.RandomLocation (AI|Navigation|GetRandomReachablePointinRadius (Transformation|GetActorLocation) 2e+03 0 0)) 0 5.0 false
      (:then
        (Variables|/Script/Engine.CharacterMovementComponent|SetMaxWalkSpeed (Variables|Character|GetCharacterMovement) (Variables|Default|GetRoam%20Speed)))
      (:OnSuccess
        (Utilities|FlowControl|Delay 1.0)
        (CallFunction|Patrol)))))

(event EventBeginPlay
  (CallFunction|StartBreathing)
  (Utilities|FlowControl|Delay 5.0)
  (Utilities|Time|ClearandInvalidateTimerbyHandle (Variables|Default|GetWalk%20To%20Location%20Time)))

(fn ConstructionScript
  (|CallParentFunction))