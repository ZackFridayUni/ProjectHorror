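; Zombie child Blueprint that makes the zombie chase its target through AI navigation.
; A custom event, with no caller in this file, starts a fast looping timer stored in WalkToPlayerTime.
; Each timer tick reissues AI MoveTo toward MyTarget and sets the walk speed.
; BeginPlay, overlap and Tick are unused placeholder nodes, and construction only calls the parent.
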(event Custom|CustomEvent
  (AI|AIMoveTo self "0, 0, 0" (Variables|Default|GetMy%20Target) 5e+01 false
    (:then
      (Variables|/Script/Engine.CharacterMovementComponent|SetMaxWalkSpeed (Variables|Character|GetCharacterMovement) 4e+02))))

(event Custom|CustomEvent_1
  (bind _returnvalue (Utilities|Time|SetTimerbyEvent (delegate Custom|CustomEvent) 0.1 true))
  (Variables|Default|SetWalk%20To%20Player%20Time _returnvalue))

(event EventBeginPlay
  (|CallParentFunction) ; This node is disabled and will not be called.\nDrag off pins to build functionality.
)

(event Collision|EventActorBeginOverlap
  (params (OtherActor :type Actor%20Object%20Reference)))

(event EventTick
  (params (DeltaSeconds :type Float%20%28single-precision%29))
  (|CallParentFunction DeltaSeconds) ; This node is disabled and will not be called.\nDrag off pins to build functionality.
)

(fn ConstructionScript
  (|CallParentFunction))