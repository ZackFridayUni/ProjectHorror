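; Parent zombie Blueprint: an AI enemy that roams, investigates noises, attacks in close range and can die.
; A looping timer walks it slowly to random reachable points until PawnSensing hears a noise, then it moves faster to that location.
; AttackRange overlap with the player starts a timer that plays the attack montage and damages MyTarget.
; Incoming damage lowers health, playing a death animation at exactly zero.
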(event OnHearNoise(PawnSensing)
  (params (Instigator :type Pawn%20Object%20Reference) (Location :type Vector%20%28by%20ref%29 :default "0, 0, 0") (Volume :type Float%20%28single-precision%29))
  ;[1 1 1] Follow Player Movement
  (Development|PrintString "Heard")
  (Utilities|Time|ClearandInvalidateTimerbyHandle (Variables|Default|GetRoam%20Timer))
  (bind _returnvalue (Utilities|Time|SetTimerbyEvent (delegate Custom|Following) 0.1))
  (Variables|Default|SetGo%20to%20Location _returnvalue))

(event OnComponentEndOverlap(AttackRange)
  (params (OverlappedComponent :type Primitive%20Component%20Object%20Reference) (OtherActor :type Actor%20Object%20Reference) (OtherComp :type Primitive%20Component%20Object%20Reference) (OtherBodyIndex :type Integer))
  ;[1 1 1] Attack Range/Damage
  (Variables|Default|SetAttackable false))

(event OnComponentBeginOverlap(AttackRange)
  (params (OverlappedComponent :type Primitive%20Component%20Object%20Reference) (OtherActor :type Actor%20Object%20Reference) (OtherComp :type Primitive%20Component%20Object%20Reference) (OtherBodyIndex :type Integer) (bFromSweep :type Boolean) (SweepResult :type Hit%20Result%20Structure%20%28by%20ref%29))
  ;[1 1 1] Attack Range/Damage
  (Variables|Default|SetAttackable true)
  (Utilities|Casting|CastToBP_FirstPersonCharacter OtherActor)
  (bind _returnvalue (Utilities|Time|SetTimerbyEvent (delegate Custom|Attack) 5.0 (Variables|Default|GetAttackable)))
  (Variables|Default|SetAttack%20Timer _returnvalue))

(event Custom|Following
  ;[1 1 1] Follow Player Movement
  (AI|AIMoveTo self (stale OnHearNoise(PawnSensing) Location) 0 5e+01 false
    (:then
      (Variables|/Script/Engine.CharacterMovementComponent|SetMaxWalkSpeed (Variables|Character|GetCharacterMovement) 2e+02)
      (Utilities|FlowControl|Delay (Variables|Default|GetDuration)))))

(event Custom|Roam%20Movement
  ;[1 1 1] Roam Movement
  (AI|AIMoveTo self (.RandomLocation (AI|Navigation|GetRandomReachablePointinRadius (Transformation|GetActorLocation) 1e+04 0 0)) 0 1e+02 false
    (:then
      (Variables|/Script/Engine.CharacterMovementComponent|SetMaxWalkSpeed (Variables|Character|GetCharacterMovement) 5e+01))))

(event Custom|Attack
  ;[1 1 1] Attack Range/Damage
  (Development|PrintString "dmg")
  (bind _returnvalue (Animation|PlayAnimMontage "/Game/Zombie/Animation/Bite/Zombie_Attack_Montage.Zombie_Attack_Montage" 1.0 "None"))
  (Variables|Default|SetAttack%20Anim%20Duration _returnvalue)
  (if (Variables|Default|GetAttackable)
    (Game|Damage|ApplyDamage (Variables|Default|GetMy%20Target) 1e+02 0 0)))

(event Custom|Roam
  ;[1 1 1] Roam Movement
  (bind _returnvalue (Utilities|Time|SetTimerbyEvent (delegate Custom|Roam%20Movement) 2.0 true false 1.0))
  (Variables|Default|SetRoam%20Timer _returnvalue))

(event Game|Damage|EventAnyDamage
  (params (Damage :type Float%20%28single-precision%29) (DamageType :type Damage%20Type%20Object%20Reference) (InstigatedBy :type Controller%20Object%20Reference) (DamageCauser :type Actor%20Object%20Reference))
  ;[1 1 1] Take Damage
  (Variables|Default|SetCurrentHealth (- (Variables|Default|GetCurrentHealth) Damage))
  (bind _output_get (Variables|Default|SetIsDead (== (Variables|Default|GetCurrentHealth) 0.0)))
  (if _output_get
    (Components|Animation|PlayAnimation (Variables|Character|GetMesh) "/Game/Zombie/Animation/Death/Zombie_Death.Zombie_Death" false)))

(event EventBeginPlay
  ;[1 1 1] Main
  (if (Variables|Default|GetHeard)
    (Utilities|Time|ClearandInvalidateTimerbyHandle (Variables|Default|GetRoam%20Timer))
    (else
      (Utilities|Time|ClearandInvalidateTimerbyHandle (Variables|Default|GetGo%20to%20Location))
      (Utilities|Time|ClearandInvalidateTimerbyHandle (Variables|Default|GetAttack%20Timer))
      (CallFunction|Roam))))

(fn ConstructionScript)

(fn GetEnemyRefrence
  (return self))