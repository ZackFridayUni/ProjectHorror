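; Sound-driven zombie enemy that roams random reachable points and chases noises heard through PawnSensing.
; A heard noise sets a looping timer that re-issues AI moves toward the sound at chase speed.
; If movement fails away from the sound, it waits, then clears the timer and resumes patrol.
; Noises also trigger an attack montage when the player overlaps AttackRange, with damage from a notify-driven forward sphere trace.
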(event OnHearNoise(PawnSensing)
  (params (Instigator :type Pawn%20Object%20Reference) (Location :type Vector%20%28by%20ref%29 :default "0, 0, 0") (Volume :type Float%20%28single-precision%29))
  ;[1 1 1] Main
  (Variables|Default|SetSound%20Location Location)
  (Variables|Default|SetHeard true)
  (Development|PrintString "Heard")
  (CallFunction|Attack)
  (CallFunction|GotoLocationOfSound))

(event OnComponentBeginOverlap(AttackRange)
  (params (OverlappedComponent :type Primitive%20Component%20Object%20Reference) (OtherActor :type Actor%20Object%20Reference) (OtherComp :type Primitive%20Component%20Object%20Reference) (OtherBodyIndex :type Integer) (bFromSweep :type Boolean) (SweepResult :type Hit%20Result%20Structure%20%28by%20ref%29))
  ;[1 1 1] Check If Player Is Nearby
  (Utilities|Casting|CastToBP_FirstPersonCharacter OtherActor)
  (Variables|Default|SetInRange? true))

(event OnComponentEndOverlap(AttackRange)
  (params (OverlappedComponent :type Primitive%20Component%20Object%20Reference) (OtherActor :type Actor%20Object%20Reference) (OtherComp :type Primitive%20Component%20Object%20Reference) (OtherBodyIndex :type Integer))
  ;[1 1 1] Check If Player Is Nearby
  (Variables|Default|SetInRange? false))

(event Custom|Following
  ;[1 1 1] Go to Location of Sound
  (AI|AIMoveTo self (Variables|Default|GetSound%20Location) 0 5e+01 false
    (:then
      (Variables|/Script/Engine.CharacterMovementComponent|SetMaxWalkSpeed (Variables|Character|GetCharacterMovement) (Variables|Default|GetSpeed%20to%20reach%20sound%20location)))
    (:OnFail
      (Development|PrintString "Movement Failed")
      (if (> (Math|Vector|Distance(Vector) (Transformation|GetActorLocation) (Variables|Default|GetSound%20Location)) 6e+01)
        (Development|PrintString "Failed 2x")
        (Utilities|FlowControl|Delay (Variables|Default|GetTime%20Before%20Bored))
        (Variables|Default|SetHeard false)
        (CallFunction|Bored)))))

(event Custom|Go%20to%20Location%20of%20Sound
  ;[1 1 1] Go to Location of Sound
  (Utilities|Time|ClearandInvalidateTimerbyHandle (Variables|Default|GetTime%20to%20reach%20random%20location))
  (bind _returnvalue (Utilities|Time|SetTimerbyEvent (delegate Custom|Following) 0.1 true))
  (Variables|Default|SetWalk%20To%20Location%20Time _returnvalue))

(event Custom|Attack
  (bind _returnvalue (Transformation|GetActorLocation))
  (bind _returnvalue_2 (Actor|GetActorOfClass "/Game/FirstPerson/Blueprints/BP_FirstPersonCharacter.BP_FirstPersonCharacter_C"))
  ;[1 1 1] Attack
  (if (Math|Boolean|ANDBoolean (Variables|Default|GetCan%20Attack?) (Variables|Default|GetHeard) (Utilities|Array|ContainsItem (Collision|GetOverlappingActors (Variables|Default|GetAttack%20Range) "/Game/FirstPerson/Blueprints/BP_FirstPersonCharacter.BP_FirstPersonCharacter_C" :!class /Script/Engine.PrimitiveComponent) _returnvalue_2))
    (Animation|Montage|PlayMontage (Variables|Character|GetMesh) "/Game/Zombie/Animation/Bite/Zombie_Attack_Montage.Zombie_Attack_Montage"
      (:then
        (Variables|Default|SetCan%20Attack? false))
      (:OnCompleted
        (Variables|Default|SetCan%20Attack? true :!label _label))
      (:OnInterrupted
        (goto _label))
      (:OnNotifyBegin
        (bind (_outhit _returnvalue_3) (Collision|SphereTraceForObjects _returnvalue (+ _returnvalue (* (Math|Vector|GetForwardVector (Transformation|GetActorRotation)) 2e+02)) 0.0 (Utilities|Array|MakeArray "ObjectTypeQuery3") false 0 "Persistent"))
        (if _returnvalue_3
          (Game|Damage|ApplyDamage (.HitActor (Collision|BreakHitResult _outhit)) 1e+01 0 0)
          (Variables|Default|SetOverlap false))))))

(event Custom|Bored
  (Utilities|Time|ClearandInvalidateTimerbyHandle (Variables|Default|GetWalk%20To%20Location%20Time))
  (CallFunction|Patrol))

(event Custom|Patrol
  ;[1 1 1] Roam Movement
  (AI|AIMoveTo self (.RandomLocation (AI|Navigation|GetRandomReachablePointinRadius (Transformation|GetActorLocation) 2e+03 0 0)) 0 5.0 false
    (:then
      (Variables|/Script/Engine.CharacterMovementComponent|SetMaxWalkSpeed (Variables|Character|GetCharacterMovement) (Variables|Default|GetRoam%20Speed)))
    (:OnSuccess
      (Utilities|FlowControl|Delay 1.0)
      (CallFunction|Patrol))))

(event EventBeginPlay
  (Utilities|Time|ClearandInvalidateTimerbyHandle (Variables|Default|GetWalk%20To%20Location%20Time))
  (CallFunction|Patrol))

(fn ConstructionScript
  (|CallParentFunction))